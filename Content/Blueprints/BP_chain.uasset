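; BP_chain is a 2D Paper2D chain actor that acts as a toggleable obstacle, raised to open and lowered to block.
; ActivateChain hides the down sprite, plays the chain-up flipbook once with a sound, and disables actor collision.
; DeactivateChain reverses that flipbook with a lowering sound and restores collision, leaving the static sprite hidden.
; Tick only prints a debug message while IsActivated is true; neither function sets that flag.
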(event `self.ReceiveTick`
  (params (DeltaSeconds :type "Float (single-precision)"))
  (if (`self.isActivated`)
    (`KismetSystemLibrary.PrintString` "Chain activated!'")))

(fn `Activate Chain`
  (`PaperSpriteComponent.SetSpriteColor` :`self` (`self.PS_chainDown`))
  (`PaperFlipbookComponent.SetLooping` (`self.FB_ChainUp`) false)
  (`PaperFlipbookComponent.SetSpriteColor` (`self.FB_ChainUp`) (struct :`R` 1.0 :`G` 1.0 :`B` 1.0 :`A` 1.0))
  (`GameplayStatics.PlaySound2D` "/Game/Assets/sfx/chainup_Cue.chainup_Cue" 1.0 1.0 0.0 null null)
  (`PaperFlipbookComponent.PlayFromStart` (`self.FB_ChainUp`))
  (`self.SetActorEnableCollision` false))

(fn `Deactivate Chain`
  (`GameplayStatics.PlaySound2D` "/Game/Assets/sfx/chaindown_Cue.chaindown_Cue" 1.0 1.0 0.0 null null)
  (`PaperFlipbookComponent.Reverse` (`self.FB_ChainUp`))
  (`self.SetActorEnableCollision` true))

(fn `UserConstructionScript`)