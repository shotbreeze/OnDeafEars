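; BP_Epiph is a Paper2D trigger that swaps Past and Future world objects when the BP_Small player character steps on it.
; On box overlap it hides its idle sprite, shows a one-shot stepped-on flipbook with a sound, and waits for that animation to finish.
; It then restores the sprite and calls Swap on every BP_Future and BP_Past actor, playing a mirror sound.
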(event `self.BOX_epiph.OnComponentBeginOverlap`
  (params (OverlappedComponent :type "PrimitiveComponent Object Reference") (OtherActor :type "Actor Object Reference") (OtherComp :type "PrimitiveComponent Object Reference") (OtherBodyIndex :type Integer) (bFromSweep :type Boolean) (SweepResult :type "HitResult Structure (by ref)"))
  (cast `/Game/Blueprints/Small/BP_Small` (`GameplayStatics.GetPlayerCharacter` 0))
  (`PaperSpriteComponent.SetSpriteColor` :`self` (`self.PS_epiph`))
  (`PaperFlipbookComponent.SetSpriteColor` (`self.PFB_epiph_stepped`) (struct :`R` 1.0 :`G` 1.0 :`B` 1.0 :`A` 1.0))
  (`PaperFlipbookComponent.SetLooping` (`self.PFB_epiph_stepped`) false)
  (`GameplayStatics.PlaySound2D` "/Game/Assets/sfx/epiph_Cue.epiph_Cue" 1.0 1.0 0.0 null null)
  (`PaperFlipbookComponent.PlayFromStart` (`self.PFB_epiph_stepped`))
  (`KismetSystemLibrary.Delay` (`PaperFlipbookComponent.GetFlipbookLength` (`self.PFB_epiph_stepped`)))
  (`PaperFlipbookComponent.SetSpriteColor` :`self` (`self.PFB_epiph_stepped`))
  (`PaperSpriteComponent.SetSpriteColor` (`self.PS_epiph`) (struct :`R` 1.0 :`G` 1.0 :`B` 1.0 :`A` 1.0))
  (`self.Swap`))

(fn `Swap`
  (bind _outactors (`GameplayStatics.GetAllActorsOfClass` "/Game/Blueprints/BP_Future.BP_Future_C"))
  (for _array_element _outactors
    (`/Game/Blueprints/BP_Future.Swap` _array_element))
  (bind _outactors_2 (`GameplayStatics.GetAllActorsOfClass` "/Game/Blueprints/BP_Past.BP_Past_C"))
  (for _array_element_2 _outactors_2
    (`/Game/Blueprints/BP_Past.Swap` _array_element_2))
  (`GameplayStatics.PlaySound2D` "/Game/Assets/sfx/mirror_Cue.mirror_Cue" 1.0 1.0 0.0 null null))

(fn `UserConstructionScript`)