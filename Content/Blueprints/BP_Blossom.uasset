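; BP_Blossom is an interactable flower that temporarily raises a linked BP_Vine when E is pressed nearby.
; A box overlap sets the proximity flag and shows a text prompt via Y scale if the player character is BP_Small.
; Pressing E swaps on/off sprites through color alpha, plays a sound and calls GoUp on the vine.
; The blossom disables its own input until a delay ends, then reverses everything with ComeDown.
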(event `self.ReceiveBeginPlay`
  (`self.EnableInput` (`GameplayStatics.GetPlayerController` 0)))

(event `Key|E` :consume false
  (params (Key :type "Key Structure"))
  (bind _vine_pointer (`self.Vine Pointer`))
  (:`Pressed`
    (if (`self.isNear`)
      (`PaperSpriteComponent.SetSpriteColor` :`self` (`self.PS_Blossom_off`))
      (`GameplayStatics.PlaySound2D` "/Game/Assets/sfx/blon_Cue.blon_Cue" 1.0 1.0 0.0 null null)
      (`PaperSpriteComponent.SetSpriteColor` (`self.PS_Blossom_on`) (struct :`R` 1.0 :`G` 1.0 :`B` 1.0 :`A` 1.0))
      (bind _asbp_vine (cast `/Game/Blueprints/BP_Vine` _vine_pointer))
      (`/Game/Blueprints/BP_Vine.Go_up` _asbp_vine)
      (`self.DisableInput` (`GameplayStatics.GetPlayerController` 0))
      (`KismetSystemLibrary.Delay` (`self.Duration`))
      (bind _asbp_vine_2 (cast `/Game/Blueprints/BP_Vine` _vine_pointer))
      (`/Game/Blueprints/BP_Vine.Come_down` _asbp_vine_2)
      (`PaperSpriteComponent.SetSpriteColor` :`self` (`self.PS_Blossom_on`))
      (`GameplayStatics.PlaySound2D` "/Game/Assets/sfx/bloff_Cue.bloff_Cue" 1.0 1.0 0.0 null null)
      (`PaperSpriteComponent.SetSpriteColor` (`self.PS_Blossom_off`) (struct :`R` 1.0 :`G` 1.0 :`B` 1.0 :`A` 1.0))
      (`self.EnableInput` (`GameplayStatics.GetPlayerController` 0)))))

(event `self.BOX_Blossom.OnComponentBeginOverlap`
  (params (OverlappedComponent :type "PrimitiveComponent Object Reference") (OtherActor :type "Actor Object Reference") (OtherComp :type "PrimitiveComponent Object Reference") (OtherBodyIndex :type Integer) (bFromSweep :type Boolean) (SweepResult :type "HitResult Structure (by ref)"))
  (cast `/Game/Blueprints/Small/BP_Small` (`GameplayStatics.GetPlayerCharacter` 0))
  (`TextRenderComponent.SetYScale` (`self.TX_blossomint`) 2.0)
  (set `self.isNear` true))

(event `self.BOX_Blossom.OnComponentEndOverlap`
  (params (OverlappedComponent :type "PrimitiveComponent Object Reference") (OtherActor :type "Actor Object Reference") (OtherComp :type "PrimitiveComponent Object Reference") (OtherBodyIndex :type Integer))
  (cast `/Game/Blueprints/Small/BP_Small` (`GameplayStatics.GetPlayerCharacter` 0))
  (`TextRenderComponent.SetYScale` (`self.TX_blossomint`) 0.0)
  (set `self.isNear` false))

(fn `UserConstructionScript`)