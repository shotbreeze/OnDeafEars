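; Flower goal actor that stays a bud until the player's BP_Small has collected its quota of memories.
; Tick polls MemCount, revealing the open sprite and glow, hiding the closed one and playing a one-time sound only when the count exactly equals MemQuota.
; Box overlap checks for at least the quota, then stops audio and opens the Welcome level, otherwise prints a prompt to collect more.
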(event `self.ReceiveTick`
  (params (DeltaSeconds :type "Float (single-precision)"))
  (bind _asbp_small (cast `/Game/Blueprints/Small/BP_Small` (`GameplayStatics.GetPlayerCharacter` 0)))
  (if (== (`/Game/Blueprints/Small/BP_Small.memCount` _asbp_small) (`self.memQuota`))
    (`PaperSpriteComponent.SetSpriteColor` (`self.PaperSprite`) (struct :`R` 1.0 :`G` 1.0 :`B` 1.0 :`A` 1.0))
    (`PaperSpriteComponent.SetSpriteColor` :`self` (`self.SP_Closed`))
    (`PaperSpriteComponent.SetSpriteColor` (`self.glow`) (struct :`R` 1.0 :`G` 1.0 :`B` 1.0 :`A` 1.0))
    (`/Engine/EditorBlueprintResources/StandardMacros.DoOnce` false
      (:`Completed`
        (`GameplayStatics.PlaySound2D` "/Game/Assets/sfx/udoneit_Cue.udoneit_Cue" 1.0 1.0 0.0 null null)))
    (else
      (`PaperSpriteComponent.SetSprite` (`self.SP_Closed`) "/Game/Assets/Sprites/SP_BUD.SP_BUD"))))

(event `self.Box.OnComponentBeginOverlap`
  (params (OverlappedComponent :type "PrimitiveComponent Object Reference") (OtherActor :type "Actor Object Reference") (OtherComp :type "PrimitiveComponent Object Reference") (OtherBodyIndex :type Integer) (bFromSweep :type Boolean) (SweepResult :type "HitResult Structure (by ref)"))
  (bind _asbp_small (cast `/Game/Blueprints/Small/BP_Small` (`GameplayStatics.GetPlayerCharacter` 0)))
  (if (>= (`/Game/Blueprints/Small/BP_Small.memCount` _asbp_small) (`self.memQuota`))
    (`KismetSystemLibrary.PrintString` "You done it")
    (`AudioMixerBlueprintLibrary.StopAudioBus` null)
    (`GameplayStatics.OpenLevel` "Welcome")
    (else
      (`KismetSystemLibrary.PrintString` "Collect more memories."))))

(fn `UserConstructionScript`)