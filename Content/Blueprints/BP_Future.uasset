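; BP_Future is an actor with a sprite, PSFuture, that toggles between a solid state and a non-colliding state.
; BeginPlay tints the sprite dark purple.
; Swap flips IsSwapped, alternating between dark purple with collision enabled and untinted white with collision disabled.
; Nothing in this Blueprint calls Swap, and Tick and overlap events are unused.
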(event `self.ReceiveBeginPlay`
  (`PaperSpriteComponent.SetSpriteColor` (`self.PS_Future`) (struct :`R` 0.323143 :`G` 0.234551 :`B` 0.456411 :`A` 1.0)))

(fn `Swap`
  (if (`self.isSwapped`)
    (set `self.isSwapped` false)
    (`PaperSpriteComponent.SetSpriteColor` (`self.PS_Future`) (struct :`R` 0.323143 :`G` 0.234551 :`B` 0.456411 :`A` 1.0))
    (`self.SetActorEnableCollision` true)
    (else
      (set `self.isSwapped` true)
      (`PaperSpriteComponent.SetSpriteColor` (`self.PS_Future`) (struct :`R` 1.0 :`G` 1.0 :`B` 1.0 :`A` 1.0))
      (`self.SetActorEnableCollision` false))))

(fn `UserConstructionScript`)