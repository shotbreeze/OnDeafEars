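; BP_Large is a playable 2D flipbook character, named Large but driven by the "Small" move and jump input actions and "small" flipbooks.
; On BeginPlay it adds the IMC_Large Enhanced Input mapping context through BP_PlayerController.
; Movement input runs along the actor's forward vector, switches between move and idle flipbooks, and flips the sprite by world rotation according to input sign.
; The jump action calls the built-in Jump.
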(event `self.ReceiveBeginPlay`
  (bind _asbp_player_controller (cast `/Game/Blueprints/BP_PlayerController` (`self.GetController`)))
  (`EnhancedInputSubsystemInterface.AddMappingContext` (pcsubsystem `EnhancedInputLocalPlayerSubsystem` _asbp_player_controller) "/Game/Blueprints/Large/IMC_Large.IMC_Large" 0 (struct)))

(event `EnhancedInput|/Game/Blueprints/Small/IA_SmallMovement`
  (params (ActionValue :type "Float (double-precision)") (ElapsedSeconds :type "Float (double-precision)") (TriggeredSeconds :type "Float (double-precision)") (InputAction :type "InputAction Object Reference" :default "/Game/Blueprints/Small/IA_SmallMovement.IA_SmallMovement"))
  (:`Triggered`
    (`self.AddMovementInput` (`self.GetActorForwardVector`) ActionValue)
    (`PaperFlipbookComponent.SetFlipbook` (`self.Sprite`) "/Game/Assets/Flipbooks/FB_smallmove.FB_smallmove")
    (if (> ActionValue 0.0)
      (`SceneComponent.K2_SetWorldRotation` (`self.Sprite`) (struct :`Yaw` -180.0) false false)
      (else
        (`SceneComponent.K2_SetWorldRotation` :`self` (`self.Sprite`)))))
  (:`Completed`
    (`PaperFlipbookComponent.SetFlipbook` (`self.Sprite`) "/Game/Assets/Flipbooks/FB_smallidle.FB_smallidle")))

(event `EnhancedInput|/Game/Blueprints/Small/IA_SmallJump`
  (params (ActionValue :type "Float (double-precision)") (ElapsedSeconds :type "Float (double-precision)") (TriggeredSeconds :type "Float (double-precision)") (InputAction :type "InputAction Object Reference" :default "/Game/Blueprints/Small/IA_SmallJump.IA_SmallJump"))
  (:`Triggered`
    (`self.Jump`)))

(fn `UserConstructionScript`)