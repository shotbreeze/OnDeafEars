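; BP_Vine is a Paper2D vine actor that can retract upward and drop back down, switching its collision off and on.
; GoUp and ComeDown swap visibility between up and down flipbooks through sprite color alpha, play the active one once from the start and play a vine sound.
; GoUp also hides the static PSVine sprite, which ComeDown does not restore.
; The event graph is empty, so nothing inside triggers either function.
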(fn `Come_down`
  (`PaperFlipbookComponent.SetSpriteColor` :`self` (`self.FB_Vine_up`))
  (`PaperFlipbookComponent.SetLooping` (`self.FB_Vine_down`) false)
  (`PaperFlipbookComponent.SetSpriteColor` (`self.FB_Vine_down`) (struct :`R` 1.0 :`G` 1.0 :`B` 1.0 :`A` 1.0))
  (`GameplayStatics.PlaySound2D` "/Game/Assets/sfx/vine_Cue.vine_Cue" 1.0 1.0 0.0 null null)
  (`PaperFlipbookComponent.PlayFromStart` (`self.FB_Vine_down`))
  (`self.SetActorEnableCollision` true))

(fn `Go_up`
  (`PaperFlipbookComponent.SetSpriteColor` :`self` (`self.FB_Vine_down`))
  (`PaperSpriteComponent.SetSpriteColor` (`self.PS_Vine`) (struct :`R` 1.0 :`G` 1.0 :`B` 1.0))
  (`PaperFlipbookComponent.SetLooping` (`self.FB_Vine_up`) false)
  (`PaperFlipbookComponent.SetSpriteColor` (`self.FB_Vine_up`) (struct :`R` 1.0 :`G` 1.0 :`B` 1.0 :`A` 1.0))
  (`GameplayStatics.PlaySound2D` "/Game/Assets/sfx/vine_Cue.vine_Cue" 1.0 1.0 0.0 null null)
  (`PaperFlipbookComponent.PlayFromStart` (`self.FB_Vine_up`))
  (`self.SetActorEnableCollision` false))

(fn `UserConstructionScript`)